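; Enemy character Blueprint that holds still briefly at spawn, shows its health on a widget bar and removes itself when dead.
; BeginPlay disables movement, restores walking after a delay and caches the BP_ENEMY_HP widget from the EnemyHealth widget component.
; Tick pushes Health into the bar as a percentage, then runs the death check shared with BeginPlay, which stops movement and destroys the actor after a delay.
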(event EventBeginPlay
  (Pawn|Components|CharacterMovement|DisableMovement (Variables|Character|GetCharacterMovement))
  (Utilities|FlowControl|Delay 5.0)
  (Pawn|Components|CharacterMovement|SetMovementMode (Variables|Character|GetCharacterMovement) "MOVE_Walking" 0)
  (bind _asbp_enemy_hp (Utilities|Casting|CastToBP_ENEMY_HP (UserInterface|GetUserWidgetObject (Variables|Default|GetEnemyHealth))))
  (Variables|Default|SetENEMY%20HP%20REF _asbp_enemy_hp)
  (if (<= (Variables|Default|GetHealth) 0.0)
    (Pawn|Components|CharacterMovement|DisableMovement (Variables|Character|GetCharacterMovement))
    (Utilities|FlowControl|Delay 2.0)
    (Actor|DestroyActor)))

(event EventTick
  (params (DeltaSeconds :type Float%20%28single-precision%29))
  (bind _enemy_hp_ref (Variables|Default|GetENEMY%20HP%20REF))
  (Utilities|IsValid _enemy_hp_ref
    (:Is%20Valid
      (Progress|SetPercent (Variables|/Game/UI/BP_ENEMY_HP.BP_ENEMY_HP_C|GetHealthBar _enemy_hp_ref) (/ (Variables|Default|GetHealth) 1e+02))
      (if (<= (Variables|Default|GetHealth) 0.0)
        (Pawn|Components|CharacterMovement|DisableMovement (Variables|Character|GetCharacterMovement))
        (Utilities|FlowControl|Delay 2.0)
        (Actor|DestroyActor)))))

(fn ConstructionScript)